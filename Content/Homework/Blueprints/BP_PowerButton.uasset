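; BP_PowerButton is an interactable button actor that switches all lamps on the map when the player presses E nearby.
; Actor overlap with a Player-tagged actor enables input from player controller 0, and end overlap disables it.
; The E key calls SwitchAllLamps, which fires the OnPressedButton event dispatcher, leaving the switching itself to bound listeners.
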(event EventSwitchAllLamps
  ;[1 1 1] Switching all lamps on the map
  (Default|CallOnPressedButton))

(event Collision|EventActorEndOverlap
  (params (OtherActor :type Actor%20Object%20Reference))
  ;[1 1 1] Proccesing begin overlap
  (if (Actor|ActorHasTag OtherActor "Player")
    (Input|DisableInput (Game|GetPlayerController 0))))

(event Collision|EventActorBeginOverlap
  (params (OtherActor :type Actor%20Object%20Reference))
  ;[1 1 1] Proccesing end overlap
  (if (Actor|ActorHasTag OtherActor "Player")
    (Input|EnableInput (Game|GetPlayerController 0))))

(event Input|KeyboardEvents|E
  (params (Key :type Key%20Structure :default "None"))
  (:Pressed
    (CallFunction|SwitchAllLamps)))

(fn ConstructionScript)